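; Game camera actor that scrolls layered background planes to create a horizontal parallax effect as it moves.
; BeginPlay creates a dynamic material instance for each of the six planes.
; Tick accumulates the camera's X movement, scaled by per-layer speed, into each material's Offset parameter.
; Layer 3 accumulates twice per tick, and layer 5's material always receives zero, so it stays static.
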(event `self.ReceiveBeginPlay`
  (bind _returnvalue (`PrimitiveComponent.CreateDynamicMaterialInstance` (`self.Plane0`) 0 "/Game/Blueprint/Material/MI_BG_0.MI_BG_0" "None"))
  (set `self.MT0` _returnvalue)
  (bind _returnvalue_2 (`PrimitiveComponent.CreateDynamicMaterialInstance` (`self.Plane1`) 0 "/Game/Blueprint/Material/MI_BG_1.MI_BG_1" "None"))
  (set `self.MT1` _returnvalue_2)
  (bind _returnvalue_3 (`PrimitiveComponent.CreateDynamicMaterialInstance` (`self.Plane2`) 0 "/Game/Blueprint/Material/MI_BG_2.MI_BG_2" "None"))
  (set `self.MT2` _returnvalue_3)
  (bind _returnvalue_4 (`PrimitiveComponent.CreateDynamicMaterialInstance` (`self.Plane3`) 0 "/Game/Blueprint/Material/MI_BG_4.MI_BG_4" "None"))
  (set `self.MT3` _returnvalue_4)
  (bind _returnvalue_5 (`PrimitiveComponent.CreateDynamicMaterialInstance` (`self.Plane4`) 0 "/Game/Blueprint/Material/MI_BG_5.MI_BG_5" "None"))
  (set `self.MT4` _returnvalue_5)
  (bind _returnvalue_6 (`PrimitiveComponent.CreateDynamicMaterialInstance` (`self.Plane5`) 0 null "None"))
  (set `self.MT5` _returnvalue_6))

(event `self.ReceiveTick`
  (params (DeltaSeconds :type "Float (single-precision)"))
  (bind _returnvalue_x (`KismetMathLibrary.BreakVector` (`self.K2_GetActorLocation`)))
  (bind _returnvalue_x_2 (`KismetMathLibrary.BreakVector` (`self.K2_GetActorLocation`)))
  (set `self.DeltaX` (- _returnvalue_x_2 (`self.CacheX`)))
  (bind _output_get (set `self.Offset0` (+ (`self.Offset0`) (* (`self.DeltaX`) (`self.ParallaxSpeed0`)))))
  (`MaterialInstanceDynamic.SetScalarParameterValue` (`self.MT0`) "Offset" _output_get)
  (bind _output_get_2 (set `self.Offset1` (+ (`self.Offset1`) (* (`self.DeltaX`) (`self.ParallaxSpeed1`)))))
  (`MaterialInstanceDynamic.SetScalarParameterValue` (`self.MT1`) "Offset" _output_get_2)
  (bind _output_get_3 (set `self.Offset2` (+ (`self.Offset2`) (* (`self.DeltaX`) (`self.ParallaxSpeed2`)))))
  (`MaterialInstanceDynamic.SetScalarParameterValue` (`self.MT2`) "Offset" _output_get_3)
  (bind _output_get_4 (set `self.Offset3` (+ (`self.Offset3`) (* (`self.DeltaX`) (`self.ParallaxSpeed3`)))))
  (`MaterialInstanceDynamic.SetScalarParameterValue` (`self.MT3`) "Offset" _output_get_4)
  (bind _output_get_5 (set `self.Offset3` (+ (`self.Offset3`) (* (`self.DeltaX`) (`self.ParallaxSpeed3`)))))
  (`MaterialInstanceDynamic.SetScalarParameterValue` (`self.MT3`) "Offset" _output_get_5)
  (bind _output_get_6 (set `self.Offset4` (+ (`self.Offset4`) (* (`self.DeltaX`) (`self.ParallaxSpeed4`)))))
  (`MaterialInstanceDynamic.SetScalarParameterValue` (`self.MT4`) "Offset" _output_get_6)
  (set `self.Offset5` (+ (`self.Offset5`) (* (`self.DeltaX`) (`self.ParallexSpeed5`))))
  (`MaterialInstanceDynamic.SetScalarParameterValue` (`self.MT5`) "Offset" 0.0)
  (set `self.CacheX` _returnvalue_x))

(fn `UserConstructionScript`)