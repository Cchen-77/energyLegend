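; BP_GJEventManager runs scripted game events, selected by the index passed to HandleEvent.
; Two dialog events start a dialog and advance it line by line on fixed delays before ending it, with the second granting the player energy partway through.
; The ending event closes the energy bar, shows the end widget, disables movement, switches to UI-only input with a hidden cursor, then plays TheEnd level sequence after a short delay.
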(event `self.HandleEvent`
  (params (index :type Integer))
  (switch `int` index
    (:`0`
      ;[1 1 1] Dialog1
      (`self.StartDialog` "/Game/Dialogs/dialog1.dialog1")
      (`self.MakeDialog`)
      (`KismetSystemLibrary.Delay` 2.0)
      (`self.MakeDialog`)
      (`KismetSystemLibrary.Delay` 2.0)
      (`self.MakeDialog`)
      (`KismetSystemLibrary.Delay` 2.0)
      (`self.MakeDialog`)
      (`KismetSystemLibrary.Delay` 2.0)
      (`self.MakeDialog`)
      (`KismetSystemLibrary.Delay` 2.0)
      (`self.MakeDialog`)
      (`KismetSystemLibrary.Delay` 2.0)
      (`self.EndDialog`))
    (:`1`
      ;[1 1 1] dialog2
      (`self.StartDialog` "/Game/Dialogs/dialog2.dialog2")
      (`self.MakeDialog`)
      (`KismetSystemLibrary.Delay` 2.0)
      (`self.MakeDialog`)
      (`KismetSystemLibrary.Delay` 2.0)
      (`self.MakeDialog`)
      (`KismetSystemLibrary.Delay` 2.0)
      (`self.MakeDialog`)
      (`KismetSystemLibrary.Delay` 2.0)
      (`self.MakeDialog`)
      (`KismetSystemLibrary.Delay` 2.0)
      (`self.MakeDialog`)
      (bind _asbp_gjcharacter_base (cast `/Game/Blueprint/Player/BP_GJCharacterBase` (`GameplayStatics.GetPlayerCharacter` 0)))
      (`GJCharacterBase.AddEnergy` _asbp_gjcharacter_base 30.0)
      (`KismetSystemLibrary.Delay` 2.0)
      (`self.MakeDialog`)
      (`KismetSystemLibrary.Delay` 2.0)
      (`self.EndDialog`))
    (:`10`
      (bind _asgjhud (cast `GJHUD` (`PlayerController.GetHUD` (`GameplayStatics.GetPlayerController` 0))))
      (`GJHUD.Close_EnergyBarWidget` _asgjhud)
      (bind _returnvalue (`|CreateWidget` "/Game/Blueprint/UI/WBP_TheEndBase.WBP_TheEndBase_C" (`GameplayStatics.GetPlayerController` 0)))
      (`UserWidget.AddToViewport` _returnvalue 0)
      (`CharacterMovementComponent.DisableMovement` (`Character.CharacterMovement` (`GameplayStatics.GetPlayerCharacter` 0)))
      (`WidgetBlueprintLibrary.SetInputMode_UIOnlyEx` (`GameplayStatics.GetPlayerController` 0) null)
      (set `PlayerController.bShowMouseCursor` false (`GameplayStatics.GetPlayerController` 0))
      (bind _outactor (`LevelSequencePlayer.CreateLevelSequencePlayer` "/Game/LevelSequence/TheEnd.TheEnd"))
      (`KismetSystemLibrary.Delay` 1.0)
      (`MovieSceneSequencePlayer.Play` (`LevelSequenceActor.SequencePlayer` _outactor)))))

(fn `UserConstructionScript`)